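; Player Megaman character for a Paper2D side-scroller, with movement, jumping, bullet shooting and a HUD widget.
; Input and landing events set a States enum that UpdateAnimation maps to sprite flipbooks; movement also turns the controller and records Facing.
; DamageSystem, also triggered by test key O, subtracts health, disables input, then knocks back or sets Dead.
; Landing after a hit plays a brief sit before restoring input; the Blink timer is never started.
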(event Custom|Blink
  ;[0 0 0] Damage System
  (Development|SetHiddeninGame (Variables|Default|GetSprite) true false)
  (Utilities|FlowControl|Delay 2.0)
  (Utilities|Time|ClearTimerbyFunctionName 0 "Blink")
  (Development|SetHiddeninGame (Variables|Default|GetSprite) false false))

(event Custom|UpdateAnimation
  ;[0 0.05938 1] Handle Animation
  (switch Utilities|FlowControl|Switch|SwitchonChar_States (Variables|Default|GetStates)
    (:NewEnumerator0
      (Sprite|SetFlipbook (Variables|Default|GetSprite) (select (> (Math|Vector|VectorLength (Transformation|GetVelocity)) 0.0) "/Game/MegamanReborn/Sprites/MegamanMannequin/A_Run.A_Run" "/Game/MegamanReborn/Sprites/MegamanMannequin/A_Idle.A_Idle")))
    (:NewEnumerator2
      (Sprite|SetFlipbook (Variables|Default|GetSprite) "/Game/MegamanReborn/Sprites/MegamanMannequin/A_Jump.A_Jump"))
    (:NewEnumerator7
      (Sprite|SetFlipbook (Variables|Default|GetSprite) "/Game/MegamanReborn/Sprites/MegamanMannequin/A_Sit.A_Sit"))
    (:NewEnumerator6
      (Sprite|SetFlipbook (Variables|Default|GetSprite) "/Game/MegamanReborn/Sprites/MegamanMannequin/A_Stand_Shoot.A_Stand_Shoot"))
    (:NewEnumerator4
      (Sprite|SetFlipbook (Variables|Default|GetSprite) "/Game/MegamanReborn/Sprites/MegamanMannequin/A_Hit.A_Hit"))
    (:NewEnumerator5
      (Sprite|SetFlipbook (Variables|Default|GetSprite) "/Game/MegamanReborn/Sprites/MegamanMannequin/A_Dead.A_Dead")
      (Input|DisableInput (Game|GetPlayerController 0)))))

(event Custom|DamageSystem
  (params (Damaging :type Float%20%28single-precision%29))
  ;[0 0 0] Damage System
  (Variables|Default|SetisHit true)
  (Input|DisableInput (Game|GetPlayerController 0))
  (bind _output_get (Variables|Default|SetHealthCurrent (- (Variables|Default|GetHealthCurrent) Damaging)))
  (if (<= _output_get 0.0)
    (Variables|Default|SetStates "NewEnumerator5")
    (else
      (Variables|Default|SetStates "NewEnumerator4")
      (Physics|AddForce (Variables|Character|GetCharacterMovement) (Math|Vector|MakeVector (* (Variables|Default|GetFacing) (Variables|Default|GetKnockback)) 0.0 2e+06)))))

(event EventOnLanded
  (params (Hit :type Hit%20Result%20Structure%20%28by%20ref%29))
  ;[0.08961 1 0] Handle Jump
  (if (Variables|Default|GetisHit)
    (Variables|Default|SetStates "NewEnumerator7")
    (CallFunction|UpdateAnimation)
    (Utilities|FlowControl|Delay 0.5)
    (Variables|Default|SetisHit false)
    (Variables|Default|SetStates "NewEnumerator0")
    (CallFunction|UpdateAnimation)
    (Input|EnableInput (Game|GetPlayerController 0))
    (else
      (Variables|Default|SetStates "NewEnumerator0")
      (CallFunction|UpdateAnimation))))

(event EventBeginPlay
  ;[0.9913 0 1] BeginPlay
  (Utilities|FlowControl|Sequence
    (:then_0
      (Class|ActorComponent|SetIsReplicated (Variables|Default|GetSprite) true))
    (:then_1
      (bind _returnvalue (UserInterface|CreateWidget "/Game/MegamanReborn/Blueprints/Widget_HUD.Widget_HUD_C" (Game|GetPlayerController 0)))
      (bind _output_get (Variables|Default|SetHealthBar _returnvalue))
      (UserInterface|Viewport|AddtoViewport _output_get 0))))

(event Input|ActionEvents|InputActionShot
  (:Pressed
    (Game|SpawnActorfromClass "/Game/MegamanReborn/Blueprints/BP_Bullet.BP_Bullet_C" (Transformation|GetWorldTransform (Variables|Default|GetArrow1)) false 0 0)
    (Variables|Default|SetStates "NewEnumerator6")
    (CallFunction|UpdateAnimation :!label _label))
  (:Released
    (Utilities|FlowControl|RetriggerableDelay 0.5)
    (Variables|Default|SetStates "NewEnumerator0")
    (goto _label)))

(event Input|ActionEvents|InputActionJump
  ;[0.08961 1 0] Handle Jump
  (:Pressed
    (Character|Jump)
    (Variables|Default|SetStates "NewEnumerator2"))
  (:Released
    (Character|StopJumping)))

(event Input|AxisEvents|InputAxisMoveRight
  (params (AxisValue :type Float%20%28single-precision%29))
  ;[1 1 1] Handle movement
  (Pawn|Input|AddMovementInput "1.000000, 0, 0" AxisValue false)
  (CallFunction|UpdateAnimation)
  (Math|Float|CompareFloat AxisValue 0.0
    (:>
      (Pawn|SetControlRotation (Pawn|GetController) (Class|KismetMathLibrary|MakeRot 0.0 0.0 0.0))
      (Variables|Default|SetFacing -1))
    (:<
      (Pawn|SetControlRotation (Pawn|GetController) (Class|KismetMathLibrary|MakeRot 0.0 1.8e+02 0.0))
      (Variables|Default|SetFacing 1))))

(event Input|KeyboardEvents|O
  ;[0.825 0 0.6039] Testing
  (:Pressed
    ;[0 0 0] Damage System
    (Variables|Default|SetisHit true)
    (Input|DisableInput (Game|GetPlayerController 0))
    (bind _output_get (Variables|Default|SetHealthCurrent (- (Variables|Default|GetHealthCurrent) (stale Custom|DamageSystem Damaging))))
    (if (<= _output_get 0.0)
      (Variables|Default|SetStates "NewEnumerator5")
      (else
        (Variables|Default|SetStates "NewEnumerator4")
        (Physics|AddForce (Variables|Character|GetCharacterMovement) (Math|Vector|MakeVector (* (Variables|Default|GetFacing) (Variables|Default|GetKnockback)) 0.0 2e+06))))))

(event Input|TouchEvents|InputTouch
  (params (Location :type Vector) (FingerIndex :type ETouchIndex%20Enum))
  ;[0.08961 1 0] Handle Jump
  (:Pressed
    (Character|Jump)
    (Variables|Default|SetStates "NewEnumerator2"))
  (:Released
    (Character|StopJumping)))

(fn ConstructionScript)